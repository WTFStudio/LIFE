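; Key-locked door that sinks when a player carrying a key overlaps it.
; On overlap it casts the player to BP_BaseCharacter and checks HasKey, printing a message if the key is missing.
; OpeningTimeline lerps the static mesh downward from its current location on each update, so the offset accumulates rather than running between fixed endpoints.
; HasKey is re-set to true during the update, so the key is not consumed.
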(event `self.ReceiveActorBeginOverlap`
  (params (OtherActor :type "Actor Object Reference"))
  (bind _returnvalue (`SceneComponent.K2_GetComponentLocation` (`self.StaticMesh`)))
  (`/Game/LIFE/Macros/MacroLibrary.IsPlayer?` OtherActor
    (:`IsPlayer`
      (bind _asbp_base_character (cast `/Game/LIFE/Characters/BaseCharacter/BP_BaseCharacter` OtherActor))
      (bind _output_get (set `self.PlayerCharacterRef` _asbp_base_character))
      (if (`/Game/LIFE/Characters/BaseCharacter/BP_BaseCharacter.HasKey?` _output_get)
        (bind (_direction _opening) (`Timeline|OpeningTimeline` :!via `PlayFromStart`)
          (:`Update`
            (`SceneComponent.K2_SetWorldLocation` (`self.StaticMesh`) (`KismetMathLibrary.VLerp` _returnvalue (+ _returnvalue (0.0 0.0 -200.0)) _opening) false false)
            (set `/Game/LIFE/Characters/BaseCharacter/BP_BaseCharacter.HasKey?` true (`self.PlayerCharacterRef`))))
        (else
          (`KismetSystemLibrary.PrintString` "You need the key"))))))

(fn `UserConstructionScript`)