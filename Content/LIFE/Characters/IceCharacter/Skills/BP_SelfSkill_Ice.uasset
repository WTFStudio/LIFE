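; BP_SelfSkill_Ice is the ice character's self-skill actor, a radial blast that knocks static mesh actors away.
; On BeginPlay it caches player 0's BP_BaseCharacter, hard-coded, and sizes its sphere from that character's CoreExplosionSkillInfo radius.
; An overlapping StaticMeshActor receives a randomized-strength, constant-falloff radial velocity impulse from the actor's location.
; That overlap also starts a delayed self-destroy, so without one the actor never destroys itself.
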(event `self.ReceiveBeginPlay`
  (bind _asbp_base_character (cast `/Game/LIFE/Characters/BaseCharacter/BP_BaseCharacter` (`GameplayStatics.GetPlayerCharacter` 0)))
  (bind _output_get (set `self.BaseCharacterRef` _asbp_base_character))
  (`SphereComponent.SetSphereRadius` (`self.Sphere`) (`.SkillRadius_34_B7A564664DAEEEB90C68A38AE5A3815F` (break `/Game/LIFE/Structures/s_SkillInfo` (`/Game/LIFE/Characters/BaseCharacter/BP_BaseCharacter.CoreExplosionSkillInfo` _output_get))) true))

(event `self.ReceiveActorBeginOverlap`
  (params (OtherActor :type "Actor Object Reference"))
  (bind _asstatic_mesh_actor (cast `StaticMeshActor` OtherActor))
  (for _array_element (`|MakeArray` (`StaticMeshActor.StaticMeshComponent` _asstatic_mesh_actor))
    (`PrimitiveComponent.AddRadialImpulse` _array_element (`self.K2_GetActorLocation`) (`.SkillRadius_34_B7A564664DAEEEB90C68A38AE5A3815F` (break `/Game/LIFE/Structures/s_SkillInfo` (`/Game/LIFE/Characters/BaseCharacter/BP_BaseCharacter.CoreExplosionSkillInfo` (`self.BaseCharacterRef`)))) (`KismetMathLibrary.RandomFloatInRange` 800.0 1200.0) "RIF_Constant" true))
  (`KismetSystemLibrary.Delay` 10.0)
  (`self.K2_DestroyActor`))

(fn `UserConstructionScript`)