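; BP_AreaSkill_Ice is a short-lived area skill actor for the ice character that wanders around the level.
; Each Tick picks random navigation-reachable points within a fixed radius of its current location and interpolates toward them without sweeping, so the heading changes every frame.
; BeginPlay starts a ten-second delay, then destroys the actor.
; The graph contains no damage or overlap logic.
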(event `self.ReceiveBeginPlay`
  (`KismetSystemLibrary.Delay` 10.0)
  (`self.K2_DestroyActor`))

(event `self.ReceiveTick`
  (params (DeltaSeconds :type "Float (single-precision)"))
  (bind _returnvalue (`KismetMathLibrary.VInterpTo` (`self.K2_GetActorLocation`) (`NavigationSystemV1.K2_GetRandomReachablePointInRadius` (`self.LastLocation`) 600.0 null null) (`GameplayStatics.GetWorldDeltaSeconds`) 3.0))
  (set `self.LastLocation` (`self.K2_GetActorLocation`))
  (`self.K2_SetActorLocation` _returnvalue)
  (set `self.LastLocation` _returnvalue))

(fn `UserConstructionScript`)