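; Base player character for a local multiplayer, twin-stick style game with elemental casters.
; On BeginPlay, PlayerInt selects the tagged PlayerStart, mesh, anim class, controller ID and skills; only fire and lightning have working skills.
; Movement follows world axes, while facing comes from gamepad stick angle or interpolated mouse-movement direction.
; Main and self skills check mana, spawn skill actors after delays and run cooldowns; self skills pause movement.
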(event `self.ReceiveBeginPlay`
  ;[1 1 1] Event Begin Play
  (`|ExecutionSequence`
    (:`then_0`
      (bind _asbp_game_mode (cast `/Game/LIFE/Blueprints/BP_GameMode` (`GameplayStatics.GetGameMode`)))
      (set `self.GameModeRef` _asbp_game_mode)
      (set `self.isPlayerAlive?` true)
      (set `self.MaxHealth` (`self.MaxHealth`))
      (set `self.MaxMana` (`self.MaxMana`)))
    (:`then_1`
      (`self.SpawnPlayers`)
      (`self.SetPlayersCharacters`))))

(event `Key|AnyKey`
  (params (Key :type "Key Structure"))
  ;[1 1 1] Check if is Gamepad Controller
  (:`Pressed`
    (set `self.IsGamepadController?` (`KismetInputLibrary.Key_IsGamepadKey` Key))))

(event `self.ReceiveTick`
  (params (DeltaSeconds :type "Float (single-precision)"))
  ;[1 1 1] Event Tick
  (`|ExecutionSequence`
    (:`then_0`
      (if (`self.isPlayerAlive?`)
        (`self.PlayerRotation`)))))

(event `InputAxis|Forward/Backword`
  (params (AxisValue :type "Float (single-precision)"))
  ;[1 1 1] Player Movement WASD and Gamepad
  (if (`self.isPlayerAlive?`)
    (`self.AddMovementInput` (1.0 0.0 0.0) AxisValue)))

(event `InputAxis|Right/Left`
  (params (AxisValue :type "Float (single-precision)"))
  ;[1 1 1] Player Movement WASD and Gamepad
  (if (`self.isPlayerAlive?`)
    (`self.AddMovementInput` (0.0 1.0 0.0) AxisValue)))

(event `InputAction|SkillCasting`
  (params (Key :type "Key Structure"))
  (:`Pressed`
    (`KismetSystemLibrary.PrintString` "Skill from character to location")))

(event `InputAction|SkillTargetLocation`
  (params (Key :type "Key Structure"))
  (:`Pressed`
    (`KismetSystemLibrary.PrintString` "Skill at location")))

(event `InputAction|SkillSelf`
  (params (Key :type "Key Structure"))
  ;[1 1 1] Switching the SelfSkill
  (:`Pressed`
    (switch `/Game/LIFE/Enums/e_SelfSkill` (`self.SelfSkillName`)
      (:`NewEnumerator1`
        (`self.CastingSelfskillImplode`))
      (:`NewEnumerator3`
        (`self.Casting SelfSkill Repulse`)))))

(event `InputAction|MainSkill`
  (params (Key :type "Key Structure"))
  ;[1 1 1] Switching the MainSkill
  (:`Pressed`
    (switch `/Game/LIFE/Enums/e_MainSkill` (`self.MainSkillName`)
      (:`NewEnumerator0`
        (`self.CastingFireballSkill`))
      (:`NewEnumerator2`
        (`self.CastLightningBolt`)))))

(event `CastingFireballSkill`
  ;[1 1 1] Cast main Skill Fireball
  (bind _enoughmana_ (`self.CheckForManaToUseSkill` (`self.FireballSkillInfo`)))
  (if (and _enoughmana_ (`self.isPlayerAlive?`) (`self.HasSkillFireball?`) (`self.IsFireballReady?`) (not (`self.HasUsedImplode?`)))
    (`self.UpdateMana` (`self.FireballSkillInfo`))
    (set `self.HasUsedFireball?` true)
    (set `self.IsFireballReady?` false)
    (`|ExecutionSequence`
      (:`then_0`
        (`KismetSystemLibrary.Delay` 0.45)
        (`|SpawnActorFromClass` "/Game/LIFE/Characters/FireCharacter/Skills/BP_MainSkillFire.BP_MainSkillFire_C" (`SceneComponent.K2_GetComponentToWorld` (`self.MainSkillSpawnPoint`)) "AlwaysSpawn" "OverrideRootScale" null null)
        (`KismetSystemLibrary.Delay` 0.7)
        (set `self.HasUsedFireball?` false))
      (:`then_1`
        (`KismetSystemLibrary.Delay` (`self.FireballCooldown`))
        (set `self.IsFireballReady?` true)))
    (else
      (`KismetSystemLibrary.PrintString` "Something is wrong" true true (struct :`G` 0.66 :`B` 1.0 :`A` 1.0) 5.0))))

(event `CastLightningBolt`
  ;[1 1 1] Cast LightningBolt
  (bind _enoughmana_ (`self.CheckForManaToUseSkill` (`self.LightningBoltSkillInfo`)))
  (if (and (`self.IsLigtningReady?`) (`self.isPlayerAlive?`) (`self.HasSkillLightningbolt?`) _enoughmana_ (not (`self.HasUsedRepulse?`)))
    (`self.UpdateMana` (`self.LightningBoltSkillInfo`))
    (set `self.HasUsedLightningBolt?` true)
    (set `self.IsLigtningReady?` false)
    (`|ExecutionSequence`
      (:`then_0`
        (`KismetSystemLibrary.Delay` 0.45)
        (`|SpawnActorFromClass` "/Game/LIFE/Characters/LightningCharacter/Skills/BP_MainSkillLightning.BP_MainSkillLightning_C" (`SceneComponent.K2_GetComponentToWorld` (`self.MainSkillSpawnPoint`)) "AlwaysSpawn" "OverrideRootScale" null null)
        (`KismetSystemLibrary.Delay` 0.7)
        (set `self.HasUsedLightningBolt?` false))
      (:`then_1`
        (`KismetSystemLibrary.Delay` (`self.LightningBoltCooldown`))
        (set `self.IsLigtningReady?` true)))
    (else
      (`KismetSystemLibrary.PrintString` "No Lightning"))))

(event `CastingSelfskillImplode`
  (bind _charactermovement (`self.CharacterMovement`))
  ;[1 1 1] Casting Selfskill Implode
  (bind _enoughmana_ (`self.CheckForManaToUseSkill` (`self.ImplodeSkillInfo`)))
  (if (and _enoughmana_ (`self.HasSkillImplode?`) (`self.IsImplodeReady?`) (`self.isPlayerAlive?`) (not (`self.HasUsedFireball?`)))
    (`self.UpdateMana` (`self.ImplodeSkillInfo`))
    (set `self.HasUsedImplode?` true)
    (set `self.IsImplodeReady?` false)
    (`|ExecutionSequence`
      (:`then_0`
        (`CharacterMovementComponent.DisableMovement` _charactermovement)
        (`MovementComponent.StopMovementImmediately` _charactermovement)
        (`KismetSystemLibrary.Delay` 1.8)
        (`|SpawnActorFromClass` "/Game/LIFE/Characters/FireCharacter/Skills/BP_SelfSkill_Fire.BP_SelfSkill_Fire_C" (`SceneComponent.K2_GetComponentToWorld` (`self.Mesh`)) "AlwaysSpawn" "OverrideRootScale" null null)
        (`KismetSystemLibrary.Delay` 1.4)
        (set `self.HasUsedImplode?` false)
        (`CharacterMovementComponent.SetMovementMode` (`self.CharacterMovement`) "MOVE_Walking" 0))
      (:`then_1`
        (`KismetSystemLibrary.Delay` 0.2)
        (set `self.IsImplodeReady?` true)))
    (else
      (`KismetSystemLibrary.PrintString` "No Implode"))))

(event `Casting SelfSkill Repulse`
  (bind _charactermovement (`self.CharacterMovement`))
  ;[1 1 1] Casting Selfskill Repulse
  (bind _enoughmana_ (`self.CheckForManaToUseSkill` (`self.RepulseSkillInfo`)))
  (if (and _enoughmana_ (`self.HasSkillRepulse?`) (`self.IsRepulseReady?`) (`self.isPlayerAlive?`) (not (`self.HasUsedLightningBolt?`)))
    (`self.UpdateMana` (`self.RepulseSkillInfo`))
    (set `self.HasUsedRepulse?` true)
    (set `self.IsRepulseReady?` false)
    (`|ExecutionSequence`
      (:`then_0`
        (`CharacterMovementComponent.DisableMovement` _charactermovement)
        (`MovementComponent.StopMovementImmediately` _charactermovement)
        (`KismetSystemLibrary.Delay` 1.8)
        (`|SpawnActorFromClass` "/Game/LIFE/Characters/FireCharacter/Skills/BP_SelfSkill_Fire.BP_SelfSkill_Fire_C" (`SceneComponent.K2_GetComponentToWorld` (`self.Mesh`)) "AlwaysSpawn" "OverrideRootScale" null null)
        (`KismetSystemLibrary.Delay` 1.4)
        (set `self.HasUsedRepulse?` false)
        (`CharacterMovementComponent.SetMovementMode` (`self.CharacterMovement`) "MOVE_Walking" 0))
      (:`then_1`
        (`KismetSystemLibrary.Delay` (`self.RepulseCooldown`))
        (set `self.IsImplodeReady?` true)))
    (else
      (`KismetSystemLibrary.PrintString` "No Repulse"))))

(fn `CheckForManaToUseSkill`
  (params (SkillInfo :type "/Game/LIFE/Structures/s_SkillInfo Structure"))
  (returns (`EnoughMana?` :type Boolean))
  (return (<= (`.SkillManaCost_31_0BC9598440002B91B9CFD5B37F0F5310` (break `/Game/LIFE/Structures/s_SkillInfo` SkillInfo)) (`self.CurrentMana`))))

(fn `GetMouseDirection`
  (returns (ReturnValue :type "Rotator Structure"))
  (bind (_returnvalue_x _returnvalue_y) (`KismetMathLibrary.BreakVector2D` (`self.GetMouseVelocity`)))
  (return (`KismetMathLibrary.RInterpTo` (`Controller.GetControlRotation` (`GameplayStatics.GetPlayerController` (`self.PlayerInt`))) (`KismetMathLibrary.MakeRotator` 0.0 0.0 (`KismetMathLibrary.DegAtan2` _returnvalue_x _returnvalue_y)) (`GameplayStatics.GetWorldDeltaSeconds`) (`self.MouseSensibility`))))

(fn `GetMouseVelocity`
  (returns (ReturnValue :type "Vector2D Structure"))
  (bind (_deltax _deltay) (`PlayerController.GetInputMouseDelta` (`GameplayStatics.GetPlayerController` (`self.PlayerInt`))))
  (return (/ (`KismetMathLibrary.MakeVector2D` _deltax _deltay) (`GameplayStatics.GetWorldDeltaSeconds`))))

(fn `GetThumbRotation`
  (returns (ReturnValue :type "Rotator Structure"))
  (return (`KismetMathLibrary.MakeRotator` 0.0 0.0 (`KismetMathLibrary.DegAtan2` (`self.GetInputAxisValue`) (`self.GetInputAxisValue`)))))

(fn `IsMouseAboveDeadzone?`
  (returns (ReturnValue :type Boolean))
  (return (> (`KismetMathLibrary.VSize2D` (`self.GetMouseVelocity`)) (`self.MouseDeadzone`))))

(fn `IsThumbAboveDeadzone?`
  (returns (ReturnValue :type Boolean))
  (return (> (`KismetMathLibrary.VSize2D` (`KismetMathLibrary.MakeVector2D` (`self.GetInputAxisValue`) (`self.GetInputAxisValue`))) (`self.ThumbDeadzone`))))

(fn `MouseRotation`
  (if (`self.IsMouseAboveDeadzone?`)
    (`Controller.SetControlRotation` (`GameplayStatics.GetPlayerController` (`self.PlayerInt`)) (`self.GetMouseDirection`))))

(fn `PlayerRotation`
  (bind _isplayeralive_ (`self.isPlayerAlive?`))
  (if (`self.IsGamepadController?`)
    (if _isplayeralive_
      (`self.ThumbRotation`))
    (elif _isplayeralive_
      (`self.MouseRotation`))))

(fn `SetPlayersCharacters`
  (bind _mesh (`self.Mesh`))
  (bind _mesh_2 (`self.Mesh`))
  ;[1 1 1] Assign character to player
  (switch `int` (`self.PlayerInt`)
    (:`0`
      ;[1 1 1] Assign the Skeletal Mesh of the character
      (`SkinnedMeshComponent.SetSkinnedAssetAndUpdate` (`self.Mesh`) "/Game/LIFE/Characters/FireCharacter/FireCharacter.FireCharacter" true)
      ;[1 1 1] Assign the Animation BP of the character
      (`SkeletalMeshComponent.SetAnimInstanceClass` (`self.Mesh`) "/Game/LIFE/Characters/FireCharacter/Animations/AnimBP_FireCharacter.AnimBP_FireCharacter_C")
      ;[1 1 1] Set Controller ID
      (`GameplayStatics.SetPlayerControllerID` null (`self.PlayerInt`))
      ;[1 1 1] Assign the skills
      (set `self.MainSkillName` "NewEnumerator0")
      (set `self.SelfSkillName` "NewEnumerator1")
      ;[1 1 1] Set skills aquired
      (set `self.HasSkillFireball?` true)
      (set `self.HasSkillImplode?` true)
      ;[1 1 1] Set skills cooldown
      (set `self.FireballCooldown` (/ (`.SkillCooldown_33_7F9A3A824905C2029EC67EAEAA3EAFA8` (break `/Game/LIFE/Structures/s_SkillInfo` (`self.FireballSkillInfo`))) 2.0))
      (set `self.ImplodeCooldown` (`.SkillCooldown_33_7F9A3A824905C2029EC67EAEAA3EAFA8` (break `/Game/LIFE/Structures/s_SkillInfo` (`self.ImplodeSkillInfo`)))))
    (:`1`
      ;[1 1 1] Set the mesh size
      (`SceneComponent.SetRelativeScale3D` _mesh (0.12 0.12 0.12))
      ;[1 1 1] Assign the Skeletal Mesh of the character
      (`SkinnedMeshComponent.SetSkinnedAssetAndUpdate` _mesh "/Game/LIFE/Characters/LightningCharacter/LightningCharacter.LightningCharacter" true)
      ;[1 1 1] Assign the Animation BP of the character
      (`SkeletalMeshComponent.SetAnimInstanceClass` (`self.Mesh`) "/Game/LIFE/Characters/LightningCharacter/Animations/Anim_BP_Lightning_Character.Anim_BP_Lightning_Character_C")
      ;[1 1 1] Set Controller ID
      (`GameplayStatics.SetPlayerControllerID` null (`self.PlayerInt`))
      ;[1 1 1] Assign the skills
      (set `self.MainSkillName` "NewEnumerator2")
      (set `self.SelfSkillName` "NewEnumerator3")
      ;[1 1 1] Set skills aquired
      (set `self.HasSkillLightningbolt?` true)
      (set `self.HasSkillRepulse?` true)
      ;[1 1 1] Set skills cooldown
      (set `self.LightningBoltCooldown` (/ (`.SkillCooldown_33_7F9A3A824905C2029EC67EAEAA3EAFA8` (break `/Game/LIFE/Structures/s_SkillInfo` (`self.LightningBoltSkillInfo`))) 2.0))
      (set `self.RepulseCooldown` (`.SkillCooldown_33_7F9A3A824905C2029EC67EAEAA3EAFA8` (break `/Game/LIFE/Structures/s_SkillInfo` (`self.RepulseSkillInfo`)))))
    (:`2`
      ;[1 1 1] Set the mesh size
      (`SceneComponent.SetRelativeScale3D` _mesh_2 (0.95 0.95 0.95))
      ;[1 1 1] Assign the Skeletal Mesh of the character
      (`SkinnedMeshComponent.SetSkinnedAssetAndUpdate` _mesh_2 "/Game/LIFE/Characters/EarthCharacter/EarthCharacter.EarthCharacter" true)
      ;[1 1 1] Assign the Animation BP of the character
      (`SkeletalMeshComponent.SetAnimInstanceClass` (`self.Mesh`) "/Game/LIFE/Characters/EarthCharacter/Animation/Anim_BP_EarthCharacter.Anim_BP_EarthCharacter_C")
      ;[1 1 1] Set Controller ID
      (`GameplayStatics.SetPlayerControllerID` null (`self.PlayerInt`))
      ;[1 1 1] Assign the skills
      (set `self.MainSkillName` "NewEnumerator3"))
    (:`3`
      ;[1 1 1] Assign the Skeletal Mesh of the character
      (`SkinnedMeshComponent.SetSkinnedAssetAndUpdate` (`self.Mesh`) "/Game/LIFE/Characters/BaseCharacter/BaseCharacter.BaseCharacter" true)
      ;[1 1 1] Assign the Animation BP of the character
      (`SkeletalMeshComponent.SetAnimInstanceClass` (`self.Mesh`) "/Game/LIFE/Characters/BaseCharacter/Animations/AnimBP_BaseCharacter.AnimBP_BaseCharacter_C")
      ;[1 1 1] Set Controller ID
      (`GameplayStatics.SetPlayerControllerID` null (`self.PlayerInt`))
      ;[1 1 1] Assign the skills
      (set `self.MainSkillName` "NewEnumerator4"))))

(fn `SpawnPlayers`
  (bind _outactors (`GameplayStatics.GetAllActorsOfClass` "/Script/Engine.PlayerStart"))
  (for _array_element _outactors
    (if (== (`PlayerStart.PlayerStartTag` _array_element) (`KismetStringLibrary.Conv_StringToName` (`KismetStringLibrary.Concat_StrStr` "Player" (`KismetStringLibrary.Conv_IntToString` (`self.PlayerInt`)))))
      (bind _output_get (set `self.SpawnLocation` (`self.GetTransform` _array_element)))
      (`self.K2_SetActorTransform` _output_get false true))))

(fn `ThumbRotation`
  (if (`self.IsThumbAboveDeadzone?`)
    (`Controller.SetControlRotation` (`GameplayStatics.GetPlayerController` (`self.PlayerInt`)) (`self.GetThumbRotation`))))

(fn `UpdateMana`
  (params (SkillInfo :type "/Game/LIFE/Structures/s_SkillInfo Structure"))
  (bind _output_get (set `self.CurrentMana` (`KismetMathLibrary.FClamp` (- (`self.CurrentMana`) (`.SkillManaCost_31_0BC9598440002B91B9CFD5B37F0F5310` (break `/Game/LIFE/Structures/s_SkillInfo` SkillInfo))) 0.0 100.0)))
  (set `self.ManaPercent` (/ _output_get (`self.MaxMana`)))
  (return))

(fn `UserConstructionScript`)