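; Projectile actor for the Earth character's main skill, apparently a thrown boulder judging by its impact effect.
; Tick spins the static mesh by incrementing one value used for roll, pitch and yaw, then runs into a Delay that destroys the actor after ten seconds.
; On hit, it spawns the impact particles slightly below the hit point, plays a 2D rock-smash sound and destroys itself.
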(event `self.ReceiveTick`
  (params (DeltaSeconds :type "Float (single-precision)"))
  (bind _result (`/Engine/EditorBlueprintResources/StandardMacros.IncrementFloat` (`self.Rotation`))
    (:`  `
      (`SceneComponent.K2_SetWorldRotation` (`self.StaticMesh`) (`KismetMathLibrary.MakeRotator` _result _result _result) false false)
      (`KismetSystemLibrary.Delay` 10.0)
      (`self.K2_DestroyActor`))))

(event `self.ReceiveHit`
  (params (MyComp :type "PrimitiveComponent Object Reference") (Other :type "Actor Object Reference") (OtherComp :type "PrimitiveComponent Object Reference") (bSelfMoved :type Boolean) (HitLocation :type "Vector Structure") (HitNormal :type "Vector Structure") (NormalImpulse :type "Vector Structure") (Hit :type "HitResult Structure (by ref)"))
  (`GameplayStatics.SpawnEmitterAtLocation` "/Game/LIFE/Characters/EarthCharacter/Skills/Particles/P_Impact_BolderToss.P_Impact_BolderToss" (`KismetMathLibrary.MakeVector` (.x HitLocation) (.y HitLocation) (- (.z HitLocation) 100.0)) (`KismetMathLibrary.MakeRotator` 0.0))
  (`GameplayStatics.PlaySound2D` "/Game/LIFE/Characters/EarthCharacter/Skills/Sounds/rock_smash.rock_smash" (`self.Volume`) (`self.Pitch`) 0.0 null null)
  (`self.K2_DestroyActor`))

(fn `UserConstructionScript`)