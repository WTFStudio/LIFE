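; Fire character self-skill actor for a core explosion that pushes nearby objects and damages NPCs.
; On BeginPlay it sizes its sphere from player 0's CoreExplosionSkillInfo, activates PushSphere, and destroys itself after three seconds.
; Overlapping static mesh actors get a randomized radial impulse, while BP_NPCs get a weaker capsule impulse plus skill damage through TakeDamage.
; Overlap branches also schedule a later destroy, which the BeginPlay timeout normally precedes.
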(event `self.ReceiveBeginPlay`
  (bind _asbp_base_character (cast `/Game/LIFE/Characters/BaseCharacter/BP_BaseCharacter` (`GameplayStatics.GetPlayerCharacter` 0)))
  (bind _output_get (set `self.BaseCharacterRef` _asbp_base_character))
  (`SphereComponent.SetSphereRadius` (`self.Sphere`) (`.SkillRadius_34_B7A564664DAEEEB90C68A38AE5A3815F` (break `/Game/LIFE/Structures/s_SkillInfo` (`/Game/LIFE/Characters/BaseCharacter/BP_BaseCharacter.CoreExplosionSkillInfo` _output_get))) true)
  (`ActorComponent.SetActive` (`self.PushSphere`) true false)
  (`KismetSystemLibrary.Delay` 3.0)
  (`self.K2_DestroyActor`))

(event `self.ReceiveActorBeginOverlap`
  (params (OtherActor :type "Actor Object Reference"))
  (`|ExecutionSequence`
    (:`then_0`
      (bind _asstatic_mesh_actor (cast `StaticMeshActor` OtherActor))
      (for _array_element (`|MakeArray` (`StaticMeshActor.StaticMeshComponent` _asstatic_mesh_actor))
        (`PrimitiveComponent.AddRadialImpulse` _array_element (`self.K2_GetActorLocation`) (`.SkillRadius_34_B7A564664DAEEEB90C68A38AE5A3815F` (break `/Game/LIFE/Structures/s_SkillInfo` (`/Game/LIFE/Characters/BaseCharacter/BP_BaseCharacter.CoreExplosionSkillInfo` (`self.BaseCharacterRef`)))) (`KismetMathLibrary.RandomFloatInRange` 800.0 1200.0) "RIF_Constant" true))
      (`KismetSystemLibrary.Delay` 10.0)
      (`self.K2_DestroyActor`))
    (:`then_1`
      (bind _asbp_npc (cast `/Game/LIFE/AI/NPC/BP_NPC` OtherActor))
      (for _array_element_2 (`|MakeArray` _asbp_npc)
        (`PrimitiveComponent.AddRadialImpulse` (`Character.CapsuleComponent` _array_element_2) (`self.K2_GetActorLocation`) (`.SkillRadius_34_B7A564664DAEEEB90C68A38AE5A3815F` (break `/Game/LIFE/Structures/s_SkillInfo` (`/Game/LIFE/Characters/BaseCharacter/BP_BaseCharacter.CoreExplosionSkillInfo` (`self.BaseCharacterRef`)))) 100.0 "RIF_Constant" true)
        (set `/Game/LIFE/AI/NPC/BP_NPC.Damage Take` (`.SkillDamage_32_AFFF0AFE4C7AB37235B562B1472C5E47` (break `/Game/LIFE/Structures/s_SkillInfo` (`/Game/LIFE/Characters/BaseCharacter/BP_BaseCharacter.CoreExplosionSkillInfo` (stale `self.ReceiveBeginPlay` _output_get)))) _asbp_npc)
        (`/Game/LIFE/AI/NPC/BP_NPC.Take damage` _asbp_npc))
      (`KismetSystemLibrary.Delay` 10.0)
      (`self.K2_DestroyActor`))))

(fn `UserConstructionScript`)