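; Shared multiplayer camera actor that zooms to suit the spread of up to four players.
; BeginPlay caches the player characters, game mode and starting camera position values.
; Each Tick branches on the game mode's MaxPlayers, setting spring arm length to the largest pairwise player distance, clamped, or a fixed length when solo.
; It also averages player locations into CenterPossition for multiple players, though this graph never moves the camera to it.
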(event `self.ReceiveBeginPlay`
  (`|ExecutionSequence`
    (:`then_0`
      (`self.GetRefToPlayers`))
    (:`then_1`
      (`self.SetCameraPosition`))
    (:`then_2`
      (bind _asbp_game_mode (cast `/Game/LIFE/Blueprints/BP_GameMode` (`GameplayStatics.GetGameMode`)))
      (set `self.GameModeRef` _asbp_game_mode))))

(event `self.ReceiveTick`
  (params (DeltaSeconds :type "Float (single-precision)"))
  (`|ExecutionSequence`
    (:`then_0`
      (switch `int` (`/Game/LIFE/Blueprints/BP_GameMode.MaxPlayers` (`self.GameModeRef`))
        (:`1`
          (`self.CalculateCameraDistanceForOnePlayer`))
        (:`2`
          (`self.CalculateCameraDistanceForTwoPlayers`))
        (:`3`
          (`self.CalculateCameraDistanceForThreePlayers`))
        (:`4`
          (`self.CalculateCameraDistanceForFourPlayers`))))
    (:`then_1`
      (`self.SetMidPoint`))))

(event `SetMidPoint`
  (switch `int` (`/Game/LIFE/Blueprints/BP_GameMode.MaxPlayers` (`self.GameModeRef`))
    (:`2`
      (bind _returnvalue (`self.CalculateMidPointForTwoPlayers`))
      (set `self.CenterPossition` _returnvalue))
    (:`3`
      (bind _returnvalue_2 (`self.CalculateMidPointForThreePlayers`))
      (set `self.CenterPossition` _returnvalue_2))
    (:`4`
      (bind _returnvalue_3 (`self.CalculateMidPointForFourPlayers`))
      (set `self.CenterPossition` _returnvalue_3))))

(fn `CalculateCameraDistanceForFourPlayers`
  (bind _player1 (`self.Player1`))
  (bind _player2 (`self.Player2`))
  (bind _player3 (`self.Player3`))
  (bind _player4 (`self.Player4`))
  (bind (_indexofmaxvalue _maxvalue) (`KismetMathLibrary.MaxOfFloatArray` (`|MakeArray` (`self.GetDistanceTo` _player1 _player2) (`self.GetDistanceTo` _player1 _player3) (`self.GetDistanceTo` _player1 _player4) (`self.GetDistanceTo` _player2 _player3) (`self.GetDistanceTo` _player2 _player4) (`self.GetDistanceTo` _player3 _player4))))
  (set `self.DistanceBetweenPlayers` _maxvalue)
  (set `SpringArmComponent.TargetArmLength` (`KismetMathLibrary.FClamp` _maxvalue (`self.MinSpringArmLenght`) (`self.MaxSpringArmLenght`)) (`self.SpringArm`)))

(fn `CalculateCameraDistanceForOnePlayer`
  (set `SpringArmComponent.TargetArmLength` 800.0 (`self.SpringArm`)))

(fn `CalculateCameraDistanceForThreePlayers`
  (bind _player1 (`self.Player1`))
  (bind _player2 (`self.Player2`))
  (bind _player3 (`self.Player3`))
  (bind (_indexofmaxvalue _maxvalue) (`KismetMathLibrary.MaxOfFloatArray` (`|MakeArray` (`self.GetDistanceTo` _player1 _player2) (`self.GetDistanceTo` _player1 _player3) (`self.GetDistanceTo` _player2 _player3))))
  (set `self.DistanceBetweenPlayers` _maxvalue)
  (set `SpringArmComponent.TargetArmLength` (`KismetMathLibrary.FClamp` _maxvalue (`self.MinSpringArmLenght`) (`self.MaxSpringArmLenght`)) (`self.SpringArm`)))

(fn `CalculateCameraDistanceForTwoPlayers`
  (bind _returnvalue (`self.GetDistanceTo` (`self.Player1`) (`self.Player2`)))
  (set `self.DistanceBetweenPlayers` _returnvalue)
  (set `SpringArmComponent.TargetArmLength` (`KismetMathLibrary.FClamp` _returnvalue (`self.MinSpringArmLenght`) (`self.MaxSpringArmLenght`)) (`self.SpringArm`)))

(fn `CalculateMidPointForFourPlayers`
  (returns (ReturnValue :type "Vector Structure"))
  (return (/ (+ (`self.K2_GetActorLocation` (`self.Player1`)) (`self.K2_GetActorLocation` (`self.Player2`)) (`self.K2_GetActorLocation` (`self.Player3`)) (`self.K2_GetActorLocation` (`self.Player4`))) (`/Game/LIFE/Blueprints/BP_GameMode.MaxPlayers` (`self.GameModeRef`)))))

(fn `CalculateMidPointForThreePlayers`
  (returns (ReturnValue :type "Vector Structure"))
  (return (/ (+ (`self.K2_GetActorLocation` (`self.Player1`)) (`self.K2_GetActorLocation` (`self.Player2`)) (`self.K2_GetActorLocation` (`self.Player3`))) (`/Game/LIFE/Blueprints/BP_GameMode.MaxPlayers` (`self.GameModeRef`)))))

(fn `CalculateMidPointForTwoPlayers`
  (returns (ReturnValue :type "Vector Structure"))
  (return (/ (+ (`self.K2_GetActorLocation` (`self.Player1`)) (`self.K2_GetActorLocation` (`self.Player2`))) (`/Game/LIFE/Blueprints/BP_GameMode.MaxPlayers` (`self.GameModeRef`)))))

(fn `GetRefToPlayers`
  (set `self.Player1` (`GameplayStatics.GetPlayerCharacter` 0))
  (set `self.Player2` (`GameplayStatics.GetPlayerCharacter` 1))
  (set `self.Player3` (`GameplayStatics.GetPlayerCharacter` 2))
  (set `self.Player4` (`GameplayStatics.GetPlayerCharacter` 3)))

(fn `SetCameraPosition`
  (bind (_returnvalue_x _returnvalue_y _returnvalue_z) (`KismetMathLibrary.BreakVector` (`self.K2_GetActorLocation`)))
  (set `self.CameraXPosition` (.x (`SceneComponent.K2_GetComponentLocation` (`self.SpringArm`))))
  (set `self.CameraYPosition` (.y (`SceneComponent.K2_GetComponentLocation` (`self.SpringArm`))))
  (set `self.CameraStartPosition` (`KismetMathLibrary.MakeVector` 0.0 0.0 _returnvalue_z)))

(fn `UserConstructionScript`)