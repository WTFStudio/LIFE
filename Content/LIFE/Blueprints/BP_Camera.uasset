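; Shared camera actor for one to four local players that keeps the group framed.
; After a short delay it reads the players from BP_GameModeTest and sets itself as the player controller's view target.
; A looping timer calls UpdateCamera, which picks per-player-count functions to size the spring arm from the largest pairwise distance, clamped, and move to the players' average position.
; Multiplayer movement is smoothed with VInterpTo, while a lone player gets a fixed arm and direct follow.
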(event `self.ReceiveBeginPlay`
  (`KismetSystemLibrary.Delay` 0.01)
  (`self.ClassSetup`)
  (`KismetSystemLibrary.K2_SetTimer` null "UpdateCamera" 0.01 true))

(event `UpdateCamera`
  (switch `int` (`KismetArrayLibrary.Array_Length` (`self.PlayersRef`))
    (:`1`
      (`self.SetArmLenghtForOnePlayer`)
      (`self.SetCameraPositionForOnePlayer`))
    (:`2`
      (`self.SetArmLenghtForTwoPlayers`)
      (`self.SetCameraPositionForTwoPlayers`))
    (:`3`
      (`self.SetArmLenghtForThreePlayers`)
      (`self.SetCameraPositionForThreePlayers`))
    (:`4`
      (`self.SetArmLenghtForFourPlayers`)
      (`self.SetCameraPositionForFourPlayers`))))

(fn `ClassSetup`
  (bind _asbp_game_mode_test (cast `/Game/LIFE/Blueprints/BP_GameModeTest` (`GameplayStatics.GetGameMode`)))
  (bind _output_get (set `self.GameModeRef` _asbp_game_mode_test))
  (set `self.PlayersRef` (`/Game/LIFE/Blueprints/BP_GameModeTest.Players` _output_get))
  (bind _outactors (`GameplayStatics.GetAllActorsOfClass` "/Script/Engine.PlayerController"))
  (`PlayerController.SetViewTargetWithBlend` _outactors self 0.0 "VTBlend_Linear" 0.0 false)
  (for (_array_element _array_index) (`self.PlayersRef`)
    (switch `int` _array_index
      (:`0`
        (set `self.Player1` _array_element))
      (:`1`
        (set `self.Player2` _array_element))
      (:`2`
        (set `self.Player3` _array_element))
      (:`3`
        (set `self.Player4` _array_element)))))

(fn `SetArmLenghtForFourPlayers`
  (bind _player1 (`self.Player1`))
  (bind _player2 (`self.Player2`))
  (bind _player3 (`self.Player3`))
  (bind _player4 (`self.Player4`))
  (set `SpringArmComponent.TargetArmLength` (`KismetMathLibrary.FClamp` (`.MaxValue` (`KismetMathLibrary.MaxOfFloatArray` (`|MakeArray` (`self.GetDistanceTo` _player1 _player2) (`self.GetDistanceTo` _player1 _player3) (`self.GetDistanceTo` _player2 _player3) (`self.GetDistanceTo` _player1 _player4) (`self.GetDistanceTo` _player3 _player4) (`self.GetDistanceTo` _player2 _player4)))) (`self.MinArmLenght`) (`self.MaxArmLenght`)) (`self.SpringArm`)))

(fn `SetArmLenghtForOnePlayer`
  (set `SpringArmComponent.TargetArmLength` (`self.DefaultArmLenght`) (`self.SpringArm`)))

(fn `SetArmLenghtForThreePlayers`
  (bind _player1 (`self.Player1`))
  (bind _player2 (`self.Player2`))
  (bind _player3 (`self.Player3`))
  (set `SpringArmComponent.TargetArmLength` (`KismetMathLibrary.FClamp` (`.MaxValue` (`KismetMathLibrary.MaxOfFloatArray` (`|MakeArray` (`self.GetDistanceTo` _player1 _player2) (`self.GetDistanceTo` _player1 _player3) (`self.GetDistanceTo` _player2 _player3)))) (`self.MinArmLenght`) (`self.MaxArmLenght`)) (`self.SpringArm`)))

(fn `SetArmLenghtForTwoPlayers`
  (set `SpringArmComponent.TargetArmLength` (`KismetMathLibrary.FClamp` (`self.GetDistanceTo` (`self.Player1`) (`self.Player2`)) (`self.MinArmLenght`) (`self.MaxArmLenght`)) (`self.SpringArm`)))

(fn `SetCameraPositionForFourPlayers`
  (set `self.TargetPosition` (/ (+ (`self.K2_GetActorLocation` (`self.Player1`)) (`self.K2_GetActorLocation` (`self.Player2`)) (`self.K2_GetActorLocation` (`self.Player3`)) (`self.K2_GetActorLocation` (`self.Player4`))) (`KismetMathLibrary.Conv_IntToDouble` (`KismetArrayLibrary.Array_Length` (`self.PlayersRef`)))))
  (`self.K2_SetActorLocation` (`KismetMathLibrary.VInterpTo` (`self.PreviousPosition`) (`self.TargetPosition`) (`GameplayStatics.GetWorldDeltaSeconds`) (`self.InterpSpeed`)))
  (set `self.PreviousPosition` (`self.K2_GetActorLocation`)))

(fn `SetCameraPositionForOnePlayer`
  (set `self.TargetPosition` (`self.K2_GetActorLocation` (`self.Player1`)))
  (`self.K2_SetActorLocation` (`self.TargetPosition`)))

(fn `SetCameraPositionForThreePlayers`
  (set `self.TargetPosition` (/ (+ (`self.K2_GetActorLocation` (`self.Player1`)) (`self.K2_GetActorLocation` (`self.Player2`)) (`self.K2_GetActorLocation` (`self.Player3`))) (`KismetMathLibrary.Conv_IntToDouble` (`KismetArrayLibrary.Array_Length` (`self.PlayersRef`)))))
  (`self.K2_SetActorLocation` (`KismetMathLibrary.VInterpTo` (`self.PreviousPosition`) (`self.TargetPosition`) (`GameplayStatics.GetWorldDeltaSeconds`) (`self.InterpSpeed`)))
  (set `self.PreviousPosition` (`self.K2_GetActorLocation`)))

(fn `SetCameraPositionForTwoPlayers`
  (set `self.TargetPosition` (/ (+ (`self.K2_GetActorLocation` (`self.Player1`)) (`self.K2_GetActorLocation` (`self.Player2`))) (`KismetMathLibrary.Conv_IntToDouble` (`KismetArrayLibrary.Array_Length` (`self.PlayersRef`)))))
  (`self.K2_SetActorLocation` (`KismetMathLibrary.VInterpTo` (`self.PreviousPosition`) (`self.TargetPosition`) (`GameplayStatics.GetWorldDeltaSeconds`) (`self.InterpSpeed`)))
  (set `self.PreviousPosition` (`self.K2_GetActorLocation`)))

(fn `UserConstructionScript`)