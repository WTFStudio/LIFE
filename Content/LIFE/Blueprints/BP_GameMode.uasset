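; Game mode that sets up local multiplayer characters and the main HUD when play begins.
; SpawnCharacters creates a local player and controller for each slot up to MaxPlayers, then spawns an indexed BP_BaseCharacter at the world origin for each controller to possess, collecting them in PlayersArray.
; BeginPlay then caches player 0's character and, if that cast succeeds, adds a single W_MainHUD to the viewport.
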(event `self.ReceiveBeginPlay`
  (`|ExecutionSequence`
    (:`then_0`
      (`self.SpawnCharacters`))
    (:`then_1`
      (bind _asbp_base_character (cast `/Game/LIFE/Characters/BaseCharacter/BP_BaseCharacter` (`GameplayStatics.GetPlayerCharacter` 0)))
      (set `self.BaseCharacterRef` _asbp_base_character))
    (:`then_2`
      (bind _returnvalue (`|CreateWidget` "/Game/LIFE/UI/W_MainHUD.W_MainHUD_C"))
      (`UserWidget.AddToViewport` _returnvalue 0))))

(fn `SpawnCharacters`
  (for _index (range (`self.MaxPlayers`))
    (bind _returnvalue (`GameplayStatics.CreatePlayer` _index))
    (set `self.PlayerControllerID` (`GameplayStatics.GetPlayerControllerID` _returnvalue))
    (set `self.PlayersIndex` _index))
  (for _index_2 (range (`self.MaxPlayers`))
    (bind _returnvalue_2 (`|SpawnActorFromClass` "/Game/LIFE/Characters/BaseCharacter/BP_BaseCharacter.BP_BaseCharacter_C" (`KismetMathLibrary.MakeTransform` (0.0 0.0 0.0)) "AlwaysSpawn" "OverrideRootScale" null _index_2 null))
    (`Controller.Possess` (`GameplayStatics.GetPlayerController` _index_2) _returnvalue_2)
    (`KismetArrayLibrary.Array_AddUnique` (`self.PlayersArray`) _returnvalue_2)))

(fn `UserConstructionScript`)