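; BP_Trap is a trap actor that damages the player after a delayed trigger.
; On overlap, it filters for a player BP_BaseCharacter, waits briefly, then activates its five particle systems and calls TakeDamage on that character with DamageAmount.
; The overlap is not rechecked after the delay, so damage applies even if the player has left the trap.
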(event `self.ReceiveActorBeginOverlap`
  (params (OtherActor :type "Actor Object Reference"))
  (`/Game/LIFE/Macros/MacroLibrary.IsPlayer?` OtherActor
    (:`IsPlayer`
      (bind _asbp_base_character (cast `/Game/LIFE/Characters/BaseCharacter/BP_BaseCharacter` OtherActor))
      (`KismetSystemLibrary.Delay` 2.0)
      (`ActorComponent.Activate` (`self.ParticleSystem1`) true)
      (`ActorComponent.Activate` (`self.ParticleSystem2`) true)
      (`ActorComponent.Activate` (`self.ParticleSystem3`) true)
      (`ActorComponent.Activate` (`self.ParticleSystem4`) true)
      (`ActorComponent.Activate` (`self.ParticleSystem5`) true)
      (`/Game/LIFE/Characters/BaseCharacter/BP_BaseCharacter.TakeDamage` _asbp_base_character (`self.DamageAmount`)))))

(fn `UserConstructionScript`)