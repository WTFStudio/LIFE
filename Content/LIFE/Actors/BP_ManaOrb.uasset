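; BP_ManaOrb is a pickup that restores mana when a player character overlaps it, but only if the full HealingAmount fits below MaxMana.
; On pickup it stores its starting transform, adds mana and plays CollectionTimeline, then destroys itself.
; The timeline lerps the orb toward the player's live location and shrinks it to zero.
; LightIntensity applies the curve value directly, leaving the stored StartingIntensity unused.
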(event `self.ReceiveActorBeginOverlap`
  (params (OtherActor :type "Actor Object Reference"))
  (`/Game/LIFE/Macros/MacroLibrary.IsPlayer?` OtherActor
    (:`IsPlayer`
      (set `self.PlayerColliding` OtherActor)
      (`self.SetStartingLocation`)
      (bind _asbp_base_character (cast `/Game/LIFE/Characters/BaseCharacter/BP_BaseCharacter` OtherActor))
      (if (`/Game/LIFE/Characters/BaseCharacter/BP_BaseCharacter.IsManaFull?` _asbp_base_character)
        _
        (elif (<= (`/Game/LIFE/Characters/BaseCharacter/BP_BaseCharacter.CurrentMana` _asbp_base_character) (- (`/Game/LIFE/Characters/BaseCharacter/BP_BaseCharacter.MaxMana` _asbp_base_character) (`self.HealingAmount`)))
          (`/Game/LIFE/Characters/BaseCharacter/BP_BaseCharacter.AddMana` _asbp_base_character (`self.HealingAmount`))
          (bind (_direction _collection _scale _intensity) (`Timeline|CollectionTimeline`)
            (:`Update`
              (`self.MoveToPlayer` _collection)
              (`self.ScaleOrb` _scale)
              (`self.LightIntensity` _intensity))
            (:`Finished`
              (`self.K2_DestroyActor`))))))))

(event `self.ReceiveTick`
  (params (DeltaSeconds :type "Float (single-precision)")))

(fn `LightIntensity`
  (params (Alpha :type "Float (double-precision)"))
  (`LightComponent.SetIntensity` (`self.PointLight`) (`KismetMathLibrary.Lerp` Alpha)))

(fn `MoveToPlayer`
  (params (Alpha :type "Float (double-precision)"))
  (`self.K2_SetActorLocation` (`KismetMathLibrary.VLerp` (`self.StartingLocation`) (`self.K2_GetActorLocation` (`self.PlayerColliding`)) Alpha)))

(fn `ScaleOrb`
  (params (Alpha :type "Float (double-precision)"))
  (`self.SetActorScale3D` (`KismetMathLibrary.VLerp` (`self.StartingScale`) (0.0 0.0 0.0) Alpha)))

(fn `SetStartingLocation`
  (set `self.StartingLocation` (`self.K2_GetActorLocation`))
  (set `self.StartingScale` (`self.GetActorScale3D`))
  (set `self.StartingIntensity` (`LightComponentBase.Intensity` (`self.PointLight`))))

(fn `UserConstructionScript`)