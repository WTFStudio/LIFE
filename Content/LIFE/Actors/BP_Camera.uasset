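; Shared-screen camera actor that frames one to four players, set as the view target for all player controllers.
; After BeginPlay, it caches players from BP_GameMode and runs a looping millisecond timer instead of Tick.
; Each update interpolates the actor toward the players' average location.
; Spring arm length follows the largest pairwise player distance, clamped between limits, or uses a default for one player.
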(event `self.ReceiveBeginPlay`
  (`KismetSystemLibrary.Delay` 0.001)
  (`self.ClassSetup`)
  (`KismetSystemLibrary.K2_SetTimer` null "UpdateCamera" 0.001 true))

(event `UpdateCamera`
  ;[1 1 1] Update Camera Zoom
  (switch `int` (`KismetArrayLibrary.Array_Length` (`self.PlayersArrayRef`))
    (:`1`
      (`self.SetArmLengthForOnePlayer`)
      ;[1 1 1] Update Camera Position
      (`self.SetCameraPositionForOnePlayers`))
    (:`2`
      (`self.SetArmLengthForTwoPlayers`)
      (`self.SetCameraPositionForTwoPlayers`))
    (:`3`
      (`self.SetArmLengthForThreePlayers`)
      (`self.SetCameraPositionForThreePlayers`))
    (:`4`
      (`self.SetArmLengthForFourPlayers`)
      (`self.SetCameraPositionForFourPlayers`))))

(fn `ClassSetup`
  (bind _asbp_game_mode (cast `/Game/LIFE/Blueprints/BP_GameMode` (`GameplayStatics.GetGameMode`)))
  (bind _output_get (set `self.GameModeRef` _asbp_game_mode))
  (set `self.PlayersArrayRef` (`/Game/LIFE/Blueprints/BP_GameMode.PlayersArray` _output_get))
  (bind _outactors (`GameplayStatics.GetAllActorsOfClass` "/Script/Engine.PlayerController"))
  (`PlayerController.SetViewTargetWithBlend` _outactors self 0.0 "VTBlend_Linear" 0.0 false)
  (for (_array_element _array_index) (`self.PlayersArrayRef`)
    (switch `int` _array_index
      (:`0`
        (set `self.Player1` _array_element))
      (:`1`
        (set `self.Player2` _array_element))
      (:`2`
        (set `self.Player3` _array_element))
      (:`3`
        (set `self.Player4` _array_element)))))

(fn `SetArmLengthForFourPlayers`
  (bind _player1 (`self.Player1`))
  (bind _player2 (`self.Player2`))
  (bind _player3 (`self.Player3`))
  (bind _player4 (`self.Player4`))
  (set `SpringArmComponent.TargetArmLength` (`KismetMathLibrary.FClamp` (`.MaxValue` (`KismetMathLibrary.MaxOfFloatArray` (`|MakeArray` (`self.GetDistanceTo` _player1 _player2) (`self.GetDistanceTo` _player1 _player3) (`self.GetDistanceTo` _player2 _player3) (`self.GetDistanceTo` _player1 _player4) (`self.GetDistanceTo` _player2 _player4) (`self.GetDistanceTo` _player3 _player4)))) (`self.MinSpringArmLength`) (`self.MaxSpringArmLength`)) (`self.SpringArm`)))

(fn `SetArmLengthForOnePlayer`
  (set `SpringArmComponent.TargetArmLength` (`self.DefaultArmLength`) (`self.SpringArm`)))

(fn `SetArmLengthForThreePlayers`
  (bind _player1 (`self.Player1`))
  (bind _player2 (`self.Player2`))
  (bind _player3 (`self.Player3`))
  (set `SpringArmComponent.TargetArmLength` (`KismetMathLibrary.FClamp` (`.MaxValue` (`KismetMathLibrary.MaxOfFloatArray` (`|MakeArray` (`self.GetDistanceTo` _player1 _player2) (`self.GetDistanceTo` _player1 _player3) (`self.GetDistanceTo` _player2 _player3)))) (`self.MinSpringArmLength`) (`self.MaxSpringArmLength`)) (`self.SpringArm`)))

(fn `SetArmLengthForTwoPlayers`
  (set `SpringArmComponent.TargetArmLength` (`KismetMathLibrary.FClamp` (`self.GetDistanceTo` (`self.Player1`) (`self.Player2`)) (`self.MinSpringArmLength`) (`self.MaxSpringArmLength`)) (`self.SpringArm`)))

(fn `SetCameraPositionForFourPlayers`
  (set `self.TargetPosition` (/ (+ (`self.K2_GetActorLocation` (`self.Player1`)) (`self.K2_GetActorLocation` (`self.Player2`)) (`self.K2_GetActorLocation` (`self.Player3`)) (`self.K2_GetActorLocation` (`self.Player4`))) (`KismetMathLibrary.Conv_IntToDouble` (`KismetArrayLibrary.Array_Length` (`self.PlayersArrayRef`)))))
  (`self.K2_SetActorLocation` (`KismetMathLibrary.VInterpTo` (`self.PreviousPosition`) (`self.TargetPosition`) (`GameplayStatics.GetWorldDeltaSeconds`) (`self.InterpSpeed`)))
  (set `self.PreviousPosition` (`self.K2_GetActorLocation`)))

(fn `SetCameraPositionForOnePlayers`
  (set `self.TargetPosition` (`self.K2_GetActorLocation` (`self.Player1`)))
  (`self.K2_SetActorLocation` (`KismetMathLibrary.VInterpTo` (`self.PreviousPosition`) (`self.TargetPosition`) (`GameplayStatics.GetWorldDeltaSeconds`) (`self.InterpSpeed`)))
  (set `self.PreviousPosition` (`self.K2_GetActorLocation`)))

(fn `SetCameraPositionForThreePlayers`
  (set `self.TargetPosition` (/ (+ (`self.K2_GetActorLocation` (`self.Player1`)) (`self.K2_GetActorLocation` (`self.Player2`)) (`self.K2_GetActorLocation` (`self.Player3`))) (`KismetMathLibrary.Conv_IntToDouble` (`KismetArrayLibrary.Array_Length` (`self.PlayersArrayRef`)))))
  (`self.K2_SetActorLocation` (`KismetMathLibrary.VInterpTo` (`self.PreviousPosition`) (`self.TargetPosition`) (`GameplayStatics.GetWorldDeltaSeconds`) (`self.InterpSpeed`)))
  (set `self.PreviousPosition` (`self.K2_GetActorLocation`)))

(fn `SetCameraPositionForTwoPlayers`
  (set `self.TargetPosition` (/ (+ (`self.K2_GetActorLocation` (`self.Player1`)) (`self.K2_GetActorLocation` (`self.Player2`))) (`KismetMathLibrary.Conv_IntToDouble` (`KismetArrayLibrary.Array_Length` (`self.PlayersArrayRef`)))))
  (`self.K2_SetActorLocation` (`KismetMathLibrary.VInterpTo` (`self.PreviousPosition`) (`self.TargetPosition`) (`GameplayStatics.GetWorldDeltaSeconds`) (`self.InterpSpeed`)))
  (set `self.PreviousPosition` (`self.K2_GetActorLocation`)))

(fn `UserConstructionScript`)