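; BP_DoubleDoorKeyRequest is a double door that opens only for a player carrying a key.
; On actor overlap, it casts the player to BP_BaseCharacter and checks HasKey, printing a message if the key is missing.
; With the key, OpeningTimeline lerps both door meshes from their current rotations toward small opposite target rotations and clears HasKey during updates, consuming the key.
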(event `self.ReceiveActorBeginOverlap`
  (params (OtherActor :type "Actor Object Reference"))
  (`/Game/LIFE/Macros/MacroLibrary.IsPlayer?` OtherActor
    (:`IsPlayer`
      (bind _asbp_base_character (cast `/Game/LIFE/Characters/BaseCharacter/BP_BaseCharacter` OtherActor))
      (bind _output_get (set `self.PlayerCharacterRef` _asbp_base_character))
      (if (`/Game/LIFE/Characters/BaseCharacter/BP_BaseCharacter.HasKey?` _output_get)
        (bind (_direction _opening) (`Timeline|OpeningTimeline` :!via `PlayFromStart`)
          (:`Update`
            (`|ExecutionSequence`
              (:`then_0`
                (`SceneComponent.K2_SetRelativeRotation` (`self.StaticMesh`) (`KismetMathLibrary.RLerp` (`SceneComponent.RelativeRotation` (`self.StaticMesh`)) (struct :`Yaw` 1.0) _opening true) false false)
                (set `/Game/LIFE/Characters/BaseCharacter/BP_BaseCharacter.HasKey?` false (`self.PlayerCharacterRef`)))
              (:`then_1`
                (`SceneComponent.K2_SetRelativeRotation` (`self.StaticMesh1`) (`KismetMathLibrary.RLerp` (`SceneComponent.RelativeRotation` (`self.StaticMesh1`)) (struct :`Yaw` -1.0) _opening true) false false)))))
        (else
          (`KismetSystemLibrary.PrintString` "You need the key"))))))

(fn `UserConstructionScript`)