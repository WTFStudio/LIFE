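; Child mutant NPC Blueprint that adds death and loot-drop behavior on top of its parent class.
; Tick runs the parent logic, then calls Death every frame while IsAlive is false.
; Death ragdolls the mesh and, after a short delay, disables capsule collision.
; A DoOnce limits the loot roll to one, which has a small chance to spawn a mana orb, otherwise a small chance for a health orb.
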(event `self.ReceiveTick`
  (params (DeltaSeconds :type "Float (single-precision)"))
  (`parent.ReceiveTick` DeltaSeconds)
  (if (not (`self.Is Alive`))
    (`self.Death`)))

(event `Death`
  (`PrimitiveComponent.SetSimulatePhysics` (`self.Mesh`) true)
  (`KismetSystemLibrary.Delay` 0.2)
  (`PrimitiveComponent.SetCollisionEnabled` (`self.CapsuleComponent`) "NoCollision")
  (`/Engine/EditorBlueprintResources/StandardMacros.DoOnce` false
    (:`Completed`
      (if (> (`KismetMathLibrary.RandomIntegerInRange` 1 10) 8)
        (`|SpawnActorFromClass` "/Game/LIFE/Actors/BP_ManaOrb.BP_ManaOrb_C" (`self.GetTransform`) "Undefined" "OverrideRootScale" null null)
        (elif (> (`KismetMathLibrary.RandomIntegerInRange` 1 10) 8)
          (`|SpawnActorFromClass` "/Game/LIFE/Actors/BP_HealthOrb.BP_HealthOrb_C" (`self.GetTransform`) "Undefined" "OverrideRootScale" null null))))))

(fn `UserConstructionScript`
  (`parent.UserConstructionScript`))