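; Boss NPC character that tracks the nearest player, makes melee attacks and has health and death handling.
; Every tick it gathers BP_BaseCharacter actors, picks the closest with a per-player-count function from GameInstance MaxPlayers, and updates its health bar widget.
; MeleeAttack sphere-traces from a collision zone between pre and post delays to damage a player.
; At zero health it stops, ragdolls, may drop a mana or health orb, then destroys itself.
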(event `self.ReceiveTick`
  (params (DeltaSeconds :type "Float (single-precision)"))
  (`|ExecutionSequence`
    (:`then_0`
      (bind _outactors (`GameplayStatics.GetAllActorsOfClass` "/Game/LIFE/Characters/BaseCharacter/BP_BaseCharacter.BP_BaseCharacter_C"))
      (bind _output_get (set `self.PlayersFound` _outactors))
      (for (_array_element _array_index) _output_get
        (switch `int` _array_index
          (:`0`
            (set `self.Player1` _array_element))
          (:`1`
            (set `self.Player2` _array_element))
          (:`2`
            (set `self.Player3` _array_element))
          (:`3`
            (set `self.Player4` _array_element)))))
    (:`then_1`
      (bind _asbp_game_instance (cast `/Game/LIFE/Blueprints/BP_GameInstance` (`GameplayStatics.GetGameInstance`)))
      (switch `int` (`/Game/LIFE/Blueprints/BP_GameInstance.MaxPlayers` _asbp_game_instance)
        (:`1`
          (`self.FindClosestPlayer1P`))
        (:`2`
          (`self.FindClosestPlayer2P`))
        (:`3`
          (`self.FindClosestPlayer3P`))
        (:`4`
          (`self.FindClosestPlayer4P`))))
    (:`then_2`
      (if (<= (`self.Current Health`) 0.0)
        (set `self.Is Alive` false)
        (if (not (`self.Is Alive`))
          (`MovementComponent.StopMovementImmediately` (`self.CharacterMovement`))
          (`CharacterMovementComponent.DisableMovement` (`self.CharacterMovement`))
          (`KismetSystemLibrary.Delay` 5.0)
          (`self.K2_DestroyActor`))))
    (:`then_3`
      (if (not (`self.Is Alive`))
        (`self.Death`)))
    (:`then_4`
      (`self.HealthPercent`))))

(event `/Game/LIFE/AI/NPC/Combat_Interface.MeleeAttack`
  (bind _returnvalue (`SceneComponent.K2_GetComponentLocation` (`self.CollisonZone`)))
  (if (`self.IsAttaking`)
    _
    (elif (`self.Is Alive`)
      (set `self.IsAttaking` true)
      (`KismetSystemLibrary.Delay` (`self.DelayPreAttack`))
      (bind _outhit (`KismetSystemLibrary.SphereTraceSingle` :`Start` _returnvalue :`End` (+ _returnvalue (* (`KismetMathLibrary.GetForwardVector` (`self.K2_GetActorRotation`)) 2.0)) :`Radius` (`SphereComponent.SphereRadius` (`self.CollisonZone`)) :`TraceChannel` "TraceTypeQuery2" :`DrawDebugType` "ForDuration"))
      (`|ExecutionSequence`
        (:`then_0`
          (bind _asbp_base_character (cast `/Game/LIFE/Characters/BaseCharacter/BP_BaseCharacter` (`.HitActor` (`GameplayStatics.BreakHitResult` _outhit))))
          (`/Game/LIFE/Characters/BaseCharacter/BP_BaseCharacter.TakeDamage` _asbp_base_character (`KismetMathLibrary.FClamp` (`self.Damage Amount`) 0.0 (`/Game/LIFE/Characters/BaseCharacter/BP_BaseCharacter.MaxHealth` _asbp_base_character)))
          (if (<= (`/Game/LIFE/Characters/BaseCharacter/BP_BaseCharacter.CurrentHealth` _asbp_base_character) 0.0)
            (set `/Game/LIFE/Characters/BaseCharacter/BP_BaseCharacter.isPlayerAlive?` false _asbp_base_character)))
        (:`then_1`
          (`KismetSystemLibrary.Delay` (`self.DelayPostAttack`))
          (set `self.IsAttaking` false))))))

(event `Take damage`
  (`|ExecutionSequence`
    (:`then_0`
      (bind _output_get (set `self.Current Health` (`KismetMathLibrary.FClamp` (- (`self.Current Health`) (`self.Damage Take`)) 0.0 (`self.Max Health`))))
      (set `self.Health%` (/ _output_get (`self.Max Health`))))
    (:`then_1`
      (`Widget.SetVisibility` (`WidgetComponent.GetUserWidgetObject` (`self.Widget`)) "Visible"))))

(event `Death`
  (`|ExecutionSequence`
    (:`then_0`
      (`PrimitiveComponent.SetSimulatePhysics` (`self.Mesh`) true)
      (`KismetSystemLibrary.Delay` 0.2)
      (`PrimitiveComponent.SetCollisionEnabled` (`self.CapsuleComponent`) "NoCollision")
      (`/Engine/EditorBlueprintResources/StandardMacros.DoOnce` false
        (:`Completed`
          (if (> (`KismetMathLibrary.RandomIntegerInRange` 1 10) 8)
            (`|SpawnActorFromClass` "/Game/LIFE/Actors/BP_ManaOrb.BP_ManaOrb_C" (`self.GetTransform`) "Undefined" "OverrideRootScale" null null)
            (elif (> (`KismetMathLibrary.RandomIntegerInRange` 1 10) 8)
              (`|SpawnActorFromClass` "/Game/LIFE/Actors/BP_HealthOrb.BP_HealthOrb_C" (`self.GetTransform`) "Undefined" "OverrideRootScale" null null))))))
    (:`then_1`
      (`Widget.SetVisibility` (`WidgetComponent.GetUserWidgetObject` (`self.Widget`)) "Hidden" :!label _label))))

(event `HealthPercent`
  (bind _ashealth_bar_bp (cast `/Game/LIFE/AI/NPC/HealthBar_BP` (`WidgetComponent.GetUserWidgetObject` (`self.Widget`))))
  (`ProgressBar.SetPercent` (`/Game/LIFE/AI/NPC/HealthBar_BP.ProgressBar_21` _ashealth_bar_bp) (`self.Health%`)))

(event `self.ReceiveBeginPlay`
  (goto _label))

(fn `FindClosestPlayer1P`
  (bind (_indexofminvalue _minvalue) (`KismetMathLibrary.MinOfFloatArray` (`|MakeArray` (`self.GetDistanceTo` (`self.Player1`) self))))
  (set `self.Closest Distance To Player` _minvalue)
  (set `self.Closest Player` _indexofminvalue))

(fn `FindClosestPlayer2P`
  (bind (_indexofminvalue _minvalue) (`KismetMathLibrary.MinOfFloatArray` (`|MakeArray` (`self.GetDistanceTo` (`self.Player1`) self) (`self.GetDistanceTo` (`self.Player2`) self))))
  (set `self.Closest Distance To Player` _minvalue)
  (set `self.Closest Player` _indexofminvalue))

(fn `FindClosestPlayer3P`
  (bind (_indexofminvalue _minvalue) (`KismetMathLibrary.MinOfFloatArray` (`|MakeArray` (`self.GetDistanceTo` (`self.Player1`) self) (`self.GetDistanceTo` (`self.Player2`) self) (`self.GetDistanceTo` (`self.Player3`) self))))
  (set `self.Closest Distance To Player` _minvalue)
  (set `self.Closest Player` _indexofminvalue))

(fn `FindClosestPlayer4P`
  (bind (_indexofminvalue _minvalue) (`KismetMathLibrary.MinOfFloatArray` (`|MakeArray` (`self.GetDistanceTo` (`self.Player1`) self) (`self.GetDistanceTo` (`self.Player2`) self) (`self.GetDistanceTo` (`self.Player3`) self) (`self.GetDistanceTo` (`self.Player4`) self))))
  (set `self.Closest Distance To Player` _minvalue)
  (set `self.Closest Player` _indexofminvalue))

(fn `UserConstructionScript`)