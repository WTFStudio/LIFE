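; BP_EnemyBaseCharacter is an enemy base character that works out which player is closest to it when play begins.
; BeginPlay reads MaxPlayers from BP_GameInstance and stores up to four found BP_BaseCharacter actors as Player1 to Player4.
; It then calls the FindClosestPlayer function for that player count, saving the index of the minimum distance in ClosestPlayer.
; The check runs only once, as Tick is empty, and nothing here acts on the result.
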(event `self.ReceiveBeginPlay`
  (`|ExecutionSequence`
    (:`then_0`
      (bind _asbp_game_instance (cast `/Game/LIFE/Blueprints/BP_GameInstance` (`GameplayStatics.GetGameInstance`)))
      (set `self.MaxPlayersRef` (`/Game/LIFE/Blueprints/BP_GameInstance.MaxPlayers` _asbp_game_instance))
      (bind _outactors (`GameplayStatics.GetAllActorsOfClass` "/Game/LIFE/Characters/BaseCharacter/BP_BaseCharacter.BP_BaseCharacter_C"))
      (bind _output_get (set `self.PlayersFound` _outactors))
      (for (_array_element _array_index) _output_get
        (switch `int` _array_index
          (:`0`
            (set `self.Player1` _array_element))
          (:`1`
            (set `self.Player2` _array_element))
          (:`2`
            (set `self.Player3` _array_element))
          (:`3`
            (set `self.Player4` _array_element)))))
    (:`then_1`
      (switch `int` (`self.MaxPlayersRef`)
        (:`1`
          (`self.FindClosestPlayer1Player`))
        (:`2`
          (`self.FindClosestPlayer2Players`))
        (:`3`
          (`self.FindClosestPlayer3Players`))
        (:`4`
          (`self.FindClosestPlayer4Players`))))))

(fn `FindClosestPlayer1Player`
  (set `self.ClosestPlayer` (`KismetMathLibrary.MinOfFloatArray` (`|MakeArray` (`self.GetDistanceTo` (`self.Player1`) self)))))

(fn `FindClosestPlayer2Players`
  (set `self.ClosestPlayer` (`KismetMathLibrary.MinOfFloatArray` (`|MakeArray` (`self.GetDistanceTo` (`self.Player1`) self) (`self.GetDistanceTo` (`self.Player2`) self)))))

(fn `FindClosestPlayer3Players`
  (set `self.ClosestPlayer` (`KismetMathLibrary.MinOfFloatArray` (`|MakeArray` (`self.GetDistanceTo` (`self.Player1`) self) (`self.GetDistanceTo` (`self.Player2`) self) (`self.GetDistanceTo` (`self.Player3`) self)))))

(fn `FindClosestPlayer4Players`
  (set `self.ClosestPlayer` (`KismetMathLibrary.MinOfFloatArray` (`|MakeArray` (`self.GetDistanceTo` (`self.Player1`) self) (`self.GetDistanceTo` (`self.Player2`) self) (`self.GetDistanceTo` (`self.Player3`) self) (`self.GetDistanceTo` (`self.Player4`) self)))))

(fn `UserConstructionScript`)